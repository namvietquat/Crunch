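; Fire variant of the Dragon Knight character on the UE4 skeleton, assembled as a visual Blueprint with no active gameplay logic.
; The Construction Script attaches the sword to the gauntlets' right-hand socket.
; It also attaches fire effects to the caped body's shoulder and chest sockets and to the head mesh's head socket.
; Attachments keep relative location and rotation, while the sword and left shoulder fire snap scale to their sockets.
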(fn `UserConstructionScript`
  (bind _ue4_body_with_cape (`self.UE4_body_with_cape`))
  (`SceneComponent.K2_AttachToComponent` (`self.UE4_sword`) (`self.UE4_gauntlets`) "hand_r" "KeepRelative" "KeepRelative" "SnapToTarget" true)
  (`SceneComponent.K2_AttachToComponent` (`self.NS_shoulder_Fire_l`) _ue4_body_with_cape "upperarm_l" "KeepRelative" "KeepRelative" "SnapToTarget" true)
  (`SceneComponent.K2_AttachToComponent` (`self.NS_shoulder_Fire_r`) _ue4_body_with_cape "upperarm_r" "KeepRelative" "KeepRelative" "KeepRelative" true)
  (`SceneComponent.K2_AttachToComponent` (`self.NS_chest_Fire`) _ue4_body_with_cape "spine_02" "KeepRelative" "KeepRelative" "KeepRelative" true)
  (`SceneComponent.K2_AttachToComponent` (`self.NS_head_Fire`) (`self.UE4 head`) "head" "KeepRelative" "KeepRelative" "KeepRelative" true))